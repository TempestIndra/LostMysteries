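; BP_PuzzleGate is a gate whose door is meant to open once enough items are collected.
; CollectItem increments the collected count, and OpenDoor plays a timeline that swings the Door's yaw to 120 degrees.
; The DoOnce-guarded check comparing the count to MaxItemsCollectable is unwired, so nothing in this graph calls OpenDoor when items are collected.
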(event Custom|Open%20Door
  (bind _door_rotation (Timeline|Open%20Door%20Anim Play)
    (:Update
      (Transformation|SetRelativeRotation (Variables|Default|GetDoor) (Math|Rotator|MakeRotator 0.0 0.0 (Math|Float|Lerp 0.0 1.2e+02 _door_rotation)) false false))))

(event Custom|Collect%20Item
  (Math|Integer|IncrementInt (Variables|Default|GetcurrentItemsCollected)))

(fn ConstructionScript)